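; Fixed-wing aircraft pawn that sets up movement of its control surfaces.
; On BeginPlay it binds three movement components, Rotation0 to Rotation2, to the aileron, elevator and rudder respectively through SetUpdatedComponent.
; Each component therefore acts on a single surface instead of the actor root.
; The graphs contain no input or flight logic, and the construction script is empty.
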(event `self.ReceiveBeginPlay`
  (`self.Setup Control Surface Rotation`))

(fn `Setup Control Surface Rotation`
  (`MovementComponent.SetUpdatedComponent` (`self.Rotation0`) (`self.Aileron`))
  (`MovementComponent.SetUpdatedComponent` (`self.Rotation1`) (`self.Elevator`))
  (`MovementComponent.SetUpdatedComponent` (`self.Rotation2`) (`self.Rudder`))
  (return))

(fn `UserConstructionScript`)